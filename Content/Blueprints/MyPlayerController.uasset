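; Player controller for a healer-style spellcasting game, managing class spells, mana and casts on party health bars.
; An Idle/Casting state gates casts on target alive, cooldown and mana, then a timer fires CastSpell, spawning a per-spell effect actor.
; Spells picked mid-cast are queued as the next selection.
; A looping timer regenerates mana; Tick and CurrentMana's RepNotify update the cast bar and mana display.
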(event Custom|TryCastSpell
  (params (PlayerToCastOn :type Health%20Bar%20Object%20Reference))
  (Variables|Default|SetselectedHealthBar PlayerToCastOn)
  (bind _cancast (CallFunction|CanCastSpell))
  (if _cancast
    (Utilities|Time|SetTimerbyFunctionName 0 "CastSpell" (.CastTime (Utilities|Struct|BreakSpellDetails (Variables|Default|GetSelectedSpell))))
    (Variables|Default|SetMyPlayerState "NewEnumerator1")
    (else
      (Development|PrintString "We have arrived at this decision"))))

(event EventBeginPlay
  (Variables|Default|SetMyPlayerState "NewEnumerator0")
  (Utilities|Time|SetTimerbyFunctionName 0 "RegenMana" 3.0 true))

(event EventTick
  (params (DeltaSeconds :type Float%20%28single-precision%29))
  (CallFunction|DisplayCastBar))

(fn ConstructionScript)

(fn SetClassDetails
  (params (Class :type Class%20Details%20Structure))
  (bind _output_get (Variables|Default|SetClass Class))
  (bind _output_get_2 (Variables|Default|SetMySpells (.Spells (Utilities|Struct|BreakClassDetails _output_get))))
  ;[1 1 1] Set the default spell to the first 1
  (CallFunction|SetSelectedSpell (.SpellName (Utilities|Struct|BreakSpellDetails (Utilities|Array|Get(acopy) _output_get_2))) (Variables|/Game/Widgets/Spells/SpellBar.SpellBar_C|GetSpellSlot_0 (Variables|/Game/Widgets/GameScreen.GameScreen_C|GetSpellBar_C (Variables|Default|GetGameScreen))))
  (bind _output_get_3 (Variables|Default|SetMaxMana (.Mana (Utilities|Struct|BreakClassDetails _output_get))))
  (Variables|Default|SetCurrentMana _output_get_3)
  (Variables|Default|SetManaRegen (.ManaRegen (Utilities|Struct|BreakClassDetails _output_get))))

(fn UseMana
  (params (ManaCost :type Integer))
  (Variables|Default|SetCurrentMana (- (Variables|Default|GetCurrentMana) ManaCost)))

(fn SetSelectedSpell
  (params (SpellName :type SpellNames%20Enum :default "NewEnumerator8") (SpellSlot :type Spell%20Slot%20Object%20Reference))
  (switch Utilities|FlowControl|Switch|SwitchonEPlayerState (Variables|Default|GetMyPlayerState)
    (:NewEnumerator0
      (Variables|Default|SetselectedSpellSlot SpellSlot)
      (for _array_element (Variables|Default|GetMySpells)
        (if (== SpellName (.SpellName (Utilities|Struct|BreakSpellDetails _array_element)))
          (Variables|Default|SetSelectedSpell _array_element))))
    (:NewEnumerator1
      (Variables|Default|SetNextSpell SpellName))))

(fn OnRepCurrentMana
  (bind _currentmana (Variables|Default|GetCurrentMana))
  (bind _maxmana (Variables|Default|GetMaxMana))
  (if (> _maxmana 0)
    (Default|DisplayMana (Variables|Default|GetGameScreen) (/ (Math|Conversions|ToFloat(Integer) _currentmana) (Math|Conversions|ToFloat(Integer) _maxmana)) (Math|Conversions|ToFloat(Integer) _currentmana))))

(fn CastSpell
  (Variables|Default|SetMyPlayerState "NewEnumerator0")
  (Default|ClearCastTIme (Variables|Default|GetGameScreen))
  (CallFunction|CreateSpell)
  ;[1 1 1] Set our next spell after we are finished casting
  (CallFunction|SetSelectedSpell (Variables|Default|GetNextSpell) (Variables|Default|GetselectedSpellSlot))
  (Variables|Default|SetNextSpell "NewEnumerator8"))

(fn CreateSpell
  (bind _selectedspell (Variables|Default|GetSelectedSpell))
  (bind _selectedspell_2 (Variables|Default|GetSelectedSpell))
  (bind _gamescreen (Variables|Default|GetGameScreen))
  (bind _selectedhealthbar (Variables|Default|GetselectedHealthBar))
  (bind (_manacost _casttime _cooldown _spellname) (Utilities|Struct|BreakSpellDetails _selectedspell))
  (CallFunction|UseMana _manacost)
  (Default|StartCD (Variables|Default|GetselectedSpellSlot))
  (switch Utilities|FlowControl|Switch|SwitchonSpellNames _spellname
    (:NewEnumerator0
      (bind _returnvalue (Game|SpawnActorfromClass "/Game/Widgets/Spells/SpellEffects/Bloom.Bloom_C" (Variables|Default|GetTransform) false 0))
      (Default|CreateEffect _returnvalue _selectedspell_2 _selectedhealthbar _gamescreen))
    (:NewEnumerator1
      (bind _returnvalue_2 (Game|SpawnActorfromClass "/Game/Widgets/Spells/SpellEffects/NaturesWarmth.NaturesWarmth_C" (Variables|Default|GetTransform) false 0))
      (Default|CreateEffect _returnvalue_2 _selectedspell_2 _selectedhealthbar _gamescreen))
    (:NewEnumerator2
      (bind _returnvalue_3 (Game|SpawnActorfromClass "/Game/Widgets/Spells/SpellEffects/Radiance.Radiance_C" (Variables|Default|GetTransform) false 0))
      (Default|CreateEffect _returnvalue_3 _selectedspell_2 _selectedhealthbar _gamescreen))
    (:NewEnumerator3
      (bind _returnvalue_4 (Game|SpawnActorfromClass "/Game/Widgets/Spells/SpellEffects/CureWounds.CureWounds_C" (Variables|Default|GetTransform) false 0))
      (Default|CreateEffect _returnvalue_4 _selectedspell_2 _selectedhealthbar _gamescreen))
    (:NewEnumerator4
      (bind _returnvalue_5 (Game|SpawnActorfromClass "/Game/Widgets/Spells/SpellEffects/ArmorOfFaith.ArmorOfFaith_C" (Variables|Default|GetTransform) false 0))
      (Default|CreateEffect _returnvalue_5 _selectedspell_2 _selectedhealthbar _gamescreen))
    (:NewEnumerator5
      (bind _returnvalue_6 (Game|SpawnActorfromClass "/Game/Widgets/Spells/SpellEffects/DivineBlessing.DivineBlessing_C" (Variables|Default|GetTransform) false 0))
      (Default|CreateEffect _returnvalue_6 _selectedspell_2 _selectedhealthbar _gamescreen))))

(fn DisplayCastBar
  (bind _selectedspell (Variables|Default|GetSelectedSpell))
  (switch Utilities|FlowControl|Switch|SwitchonEPlayerState (Variables|Default|GetMyPlayerState)
    (:NewEnumerator1
      (if (> (.casttime _selectedspell) 0.0)
        (Default|DisplayCastTime (Variables|Default|GetGameScreen) (/ (Class|KismetSystemLibrary|GetTimerElapsedTime 0 "CastSpell") (.casttime _selectedspell)))
        (return)))))

(fn RegenMana
  (if (> (+ (Variables|Default|GetCurrentMana) (* 1 (Math|Float|Floor (Variables|Default|GetManaRegen)))) (Variables|Default|GetMaxMana))
    (Variables|Default|SetCurrentMana (Variables|Default|GetMaxMana))
    (else
      (Variables|Default|SetCurrentMana (+ (Variables|Default|GetCurrentMana) (* 1 (Math|Float|Floor (Variables|Default|GetManaRegen))))))))

(fn CanCastSpell
  (bind _selectedspellslot (Variables|Default|GetselectedSpellSlot))
  (Utilities|IsValid _selectedspellslot
    (:Is%20Valid
      (if (Variables|/Game/Widgets/Party/HealthBar.HealthBar_C|GetbDeceased (Variables|Default|GetselectedHealthBar))
        (Development|PrintString "Player Is dead")
        (LocalVariables|SetbCanCast false)
        (else
          (switch Utilities|FlowControl|Switch|SwitchonEPlayerState (Variables|Default|GetMyPlayerState)
            (:NewEnumerator0
              (bind _finished (Default|IsCdComplete _selectedspellslot))
              (if _finished
                (bind _hasmana (CallFunction|HasMana))
                (if _hasmana
                  (LocalVariables|SetbCanCast true)
                  (else
                    (Development|PrintString "Out of mana")
                    (LocalVariables|SetbCanCast false)))
                (else
                  (Development|PrintString "Spell on CD")
                  (LocalVariables|SetbCanCast false))))
            (:NewEnumerator1
              (Development|PrintString "Still Casting a spell")
              (LocalVariables|SetbCanCast false))))))
    (:Is%20Not%20Valid
      (Development|PrintString "spell slot not valid")
      (LocalVariables|SetbCanCast false)))
  (return (LocalVariables|GetbCanCast)))

(fn HasMana
  (bind _currentmana (Variables|Default|GetCurrentMana))
  (LocalVariables|SetbhasMana true)
  (if (>= _currentmana (.ManaCost (Utilities|Struct|BreakSpellDetails (Variables|Default|GetSelectedSpell))))
    (if (> _currentmana 0)
      _
      (else
        (LocalVariables|SetbhasMana false :!label _label)))
    (else
      (goto _label)))
  (return (LocalVariables|GetbhasMana)))
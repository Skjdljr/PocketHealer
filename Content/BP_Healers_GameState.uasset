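; BP_Healers_GameState is the game state that builds the set of quest contracts when play begins.
; On BeginPlay it loops over every row of the QuestContractLibrary data table held by BP_Healers_GameMode.
; For each row found, it spawns a QuestContractClass actor at the origin, copies the row into it and adds it to the QuestContracts array.
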(event EventBeginPlay
  (bind _returnvalue (Game|GetGameMode))
  (bind _asbp_healers_game_mode (Utilities|Casting|CastToBP_Healers_GameMode _returnvalue))
  (bind _questcontractlibrary (Variables|/Script/HealersQuest.Healers_GameMode|GetQuestContractLibrary _asbp_healers_game_mode))
  (bind _outrownames (DataTable|GetDataTableRowNames _questcontractlibrary))
  (for _array_element _outrownames
    (bind _returnvalue_2 (Utilities|GetDataTableRow _questcontractlibrary _array_element)
      (:then
        (bind _returnvalue_3 (Game|SpawnActorfromClass (Variables|Default|GetQuestContractClass) (Math|Transform|MakeTransform "0, 0, 0") "Undefined" 0 0))
        (bind _ashealers_quest_contract (Utilities|Casting|CastToHealers_QuestContract _returnvalue_3))
        (Variables|/Script/HealersQuest.Healers_QuestContract|SetQuestContract _ashealers_quest_contract _returnvalue_2)
        (Utilities|Array|AddUnique (Variables|Default|GetQuestContracts) _ashealers_quest_contract)))))

(event EventTick
  (params (DeltaSeconds :type Float%20%28single-precision%29)))

(fn ConstructionScript)